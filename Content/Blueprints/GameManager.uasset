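; GameManager actor that runs a Breakout level: block counting, ball spawning, win and lose states, and level flow.
; Blocks report creation and breakage to trigger the clear widget, while misses with no balls left trigger game over.
; A single Action entry point spawns a ball, reloads the level after game over, or opens the next level.
; Remaining balls update the HUD widget and carry over, plus one, through BreakoutGameInstance.
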(event EventBeginPlay
  (bind _returnvalue (UserInterface|CreateWidget "/Game/Widgets/GameInformation.GameInformation_C"))
  (Variables|Default|SetGameInformationWidget _returnvalue)
  (UserInterface|Viewport|AddtoViewport _returnvalue 0)
  (bind _asbreakout_game_instance (Utilities|Casting|CastToBreakoutGameInstance (Game|GetGameInstance))
    (:then
      (if (Default|IsValidBallNum _asbreakout_game_instance)
        (Variables|Default|SetLeftBallNum (Variables|/Game/Blueprints/BreakoutGameInstance.BreakoutGameInstance_C|GetLeftBallNum _asbreakout_game_instance))))
    (:CastFailed
      _))
  (CallFunction|RefreshGameInformation))

(event Collision|EventActorBeginOverlap
  (params (OtherActor :type Actor%20Object%20Reference)))

(event EventTick
  (params (DeltaSeconds :type Float%20%28single-precision%29)))

(fn ConstructionScript)

(fn AddBlockNum
  (Variables|Default|SetBlockNum (+ (Variables|Default|GetBlockNum) 1)))

(fn AddBrokenBlockNum
  (Variables|Default|SetBrokenBlockNum (+ (Variables|Default|GetBrokenBlockNum) 1))
  (if (not (Variables|Default|GetIsGameOver))
    (if (not (Variables|Default|GetIsCleared))
      (if (<= (CallFunction|GetLeftBlockNum) 0)
        (Variables|Default|SetIsCleared true)
        (CallFunction|ViewGameClearWidget)))))

(fn GetLeftBlockNum
  (return (- (Variables|Default|GetBlockNum) (Variables|Default|GetBrokenBlockNum))))

(fn ViewGameClearWidget
  (bind _returnvalue (UserInterface|CreateWidget "/Game/UI/ClearWidget.ClearWidget_C"))
  (UserInterface|Viewport|AddtoViewport _returnvalue 0))

(fn ViewGameOverWidget
  (bind _returnvalue (UserInterface|CreateWidget "/Game/UI/GameOverWidget.GameOverWidget_C"))
  (UserInterface|Viewport|AddtoViewport _returnvalue 0))

(fn MissCount
  (if (not (Variables|Default|GetIsCleared))
    (if (not (Variables|Default|GetIsGameOver))
      (Variables|Default|SetIsBallSpawned false)
      (if (<= (Variables|Default|GetLeftBallNum) 0)
        (Variables|Default|SetIsGameOver true)
        (CallFunction|ViewGameOverWidget)))))

(fn SpawnBall
  (if (not (Variables|Default|GetIsBallSpawned))
    (if (> (Variables|Default|GetLeftBallNum) 0)
      (Game|SpawnActorfromClass "/Game/Blueprints/Ball.Ball_C" (Transformation|GetActorTransform (Variables|Default|GetSpawnLocationActor)) "Undefined" "MultiplyWithRoot" 0 0)
      (Variables|Default|SetIsBallSpawned true)
      (Variables|Default|SetLeftBallNum (- (Variables|Default|GetLeftBallNum) 1))
      (CallFunction|RefreshGameInformation))))

(fn Action
  (if (Variables|Default|GetIsGameOver)
    (CallFunction|LevelReset)
    (elif (Variables|Default|GetIsCleared)
      (CallFunction|OpenNextLevel)
      (else
        (CallFunction|SpawnBall)))))

(fn LevelReset
  (bind _returnvalue (Game|GetCurrentLevelName true))
  (Game|OpenLevel(byName) (Utilities|String|StringToName _returnvalue)))

(fn GetLeftBallNum
  (return (Variables|Default|GetLeftBallNum)))

(fn RefreshGameInformation
  (Variables|/Game/Widgets/GameInformation.GameInformation_C|SetLeftBallNum (Variables|Default|GetGameInformationWidget) (Variables|Default|GetLeftBallNum)))

(fn OpenNextLevel
  (bind _asbreakout_game_instance (Utilities|Casting|CastToBreakoutGameInstance (Game|GetGameInstance))
    (:then
      (Variables|/Game/Blueprints/BreakoutGameInstance.BreakoutGameInstance_C|SetLeftBallNum _asbreakout_game_instance (+ (Variables|Default|GetLeftBallNum) 1)))
    (:CastFailed
      _))
  (Game|OpenLevel(byName) (Variables|Default|GetNextLevelName)))