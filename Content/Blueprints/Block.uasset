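; Breakable block actor for a ball-and-block game that loses one HP each time a Ball hits its Cube.
; It shows HP as text and tints a dynamic material, created in the construction script, from a color table indexed by HP.
; It registers with the GameManager on BeginPlay.
; At zero HP, a DoOnce reports the break to the GameManager, then destroys the actor after a short delay.
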(event OnComponentHit(Cube)
  (params (HitComponent :type Primitive%20Component%20Object%20Reference) (OtherActor :type Actor%20Object%20Reference) (OtherComp :type Primitive%20Component%20Object%20Reference) (NormalImpulse :type Vector :default "0, 0, 0") (Hit :type Hit%20Result%20Structure%20%28by%20ref%29))
  (Utilities|Casting|CastToBall OtherActor)
  (bind _output_get (Variables|Default|SetHp (- (Variables|Default|GetHp) 1)))
  (CallFunction|ReloadHp)
  (if (<= _output_get 0)
    (Utilities|FlowControl|DoOnce false
      (:Completed
        (bind _returnvalue (Actor|GetActorOfClass "/Game/Blueprints/GameManager.GameManager_C"))
        (Default|AddBrokenBlockNum _returnvalue)
        (Utilities|FlowControl|Delay 0.05)
        (Actor|DestroyActor)))))

(event EventBeginPlay
  (bind _returnvalue (Actor|GetActorOfClass "/Game/Blueprints/GameManager.GameManager_C"))
  (Default|AddBlockNum _returnvalue)
  (CallFunction|ReloadHp))

(event Collision|EventActorBeginOverlap
  (params (OtherActor :type Actor%20Object%20Reference)))

(event EventTick
  (params (DeltaSeconds :type Float%20%28single-precision%29)))

(fn ConstructionScript
  (bind _returnvalue (Rendering|Material|CreateDynamicMaterialInstance (Variables|Default|GetCube) 0 0 "None" :!class /Script/Engine.PrimitiveComponent))
  (Variables|Default|SetMaterialInstance _returnvalue))

(fn ReloadHp
  (bind _colortable (Variables|Default|GetColorTable))
  (bind _hp (Variables|Default|GetHp))
  (bind _returnvalue (- _hp 1))
  (Rendering|Components|TextRender|SetText (Variables|Default|GetHpText) (Utilities|Text|ToText(Integer) (Variables|Default|GetHp)))
  (if (Utilities|Array|IsValidIndex _colortable _returnvalue)
    (Rendering|Material|SetVectorParameterValue (Variables|Default|GetMaterialInstance) "BaseColor" (Utilities|Array|Get(acopy) _colortable _returnvalue) :!class /Script/Engine.MaterialInstanceDynamic)))