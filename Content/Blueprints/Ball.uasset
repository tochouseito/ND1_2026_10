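; Breakout ball actor that moves along a normalized direction at a set speed using a swept offset each tick.
; On hit, a paddle's top face sets the new direction from its aim function at the impact point; any other surface mirrors the direction by the hit normal.
; Every hit plays a knock sound.
; Overlapping a MissArea-tagged component reports a miss to the GameManager and destroys the ball.
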(event OnComponentHit(Sphere)
  (params (HitComponent :type Primitive%20Component%20Object%20Reference) (OtherActor :type Actor%20Object%20Reference) (OtherComp :type Primitive%20Component%20Object%20Reference) (NormalImpulse :type Vector :default "0, 0, 0") (Hit :type Hit%20Result%20Structure%20%28by%20ref%29))
  (bind (_bblockinghit _binitialoverlap _time _distance _location _impactpoint _normal _impactnormal) (Collision|BreakHitResult Hit))
  (bind _aspaddle (Utilities|Casting|CastToPaddle OtherActor)
    (:then
      (if (> (Math|Vector|DotProduct _impactnormal "0,0,1") 0.5)
        (Variables|Default|SetDirection (Default|GetAimDirection _aspaddle _impactpoint))
        (else
          (Variables|Default|SetDirection (Math|Vector|MirrorVectorbyNormal (Variables|Default|GetDirection) _impactnormal) :!label _label))))
    (:CastFailed
      (goto _label)))
  (Audio|PlaySound2D "/Game/Audio/Breakout_SE_Knock/Breakout_SE_Knock.Breakout_SE_Knock" 1.0 1.0 0.0 0 0))

(event OnComponentBeginOverlap(Sphere)
  (params (OverlappedComponent :type Primitive%20Component%20Object%20Reference) (OtherActor :type Actor%20Object%20Reference) (OtherComp :type Primitive%20Component%20Object%20Reference) (OtherBodyIndex :type Integer) (bFromSweep :type Boolean) (SweepResult :type Hit%20Result%20Structure%20%28by%20ref%29))
  (if (Components|ComponentHasTag OtherComp "MissArea")
    (bind _returnvalue (Actor|GetActorOfClass "/Game/Blueprints/GameManager.GameManager_C"))
    (Default|MissCount _returnvalue)
    (Actor|DestroyActor)))

(event EventBeginPlay
  (Variables|Default|SetDirection (Math|Vector|Normalize (Variables|Default|GetDirection))))

(event Collision|EventActorBeginOverlap
  (params (OtherActor :type Actor%20Object%20Reference)))

(event EventTick
  (params (DeltaSeconds :type Float%20%28single-precision%29))
  (Transformation|AddActorWorldOffset (* (Variables|Default|GetDirection) (* (Variables|Default|GetSpeed) DeltaSeconds)) true))

(fn ConstructionScript)