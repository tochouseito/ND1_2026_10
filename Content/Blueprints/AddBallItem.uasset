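; AddBallItem is a falling pickup that adds a ball when the paddle catches it.
; Tick moves it along Z by FallSpeed scaled by delta time, without sweeping.
; On overlap with a Paddle it finds the GameManager via GetActorOfClass, calls GenerateBall and destroys itself.
; Overlapping a TriggerBox destroys it without spawning a ball.
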(event EventBeginPlay)

(event Collision|EventActorBeginOverlap
  (params (OtherActor :type Actor%20Object%20Reference))
  (Utilities|Casting|CastToPaddle OtherActor
    (:then
      (bind _returnvalue (Actor|GetActorOfClass "/Game/Blueprints/GameManager.GameManager_C"))
      (Default|GenerateBall _returnvalue)
      (Actor|DestroyActor))
    (:CastFailed
      (Utilities|Casting|CastToTriggerBox OtherActor)
      (Actor|DestroyActor))))

(event EventTick
  (params (DeltaSeconds :type Float%20%28single-precision%29))
  (Transformation|AddActorWorldOffset (Math|Vector|MakeVector 0.0 0.0 (* (Variables|Default|GetFallSpeed) DeltaSeconds))))

(fn ConstructionScript)